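; Factory dispenser actor that endlessly squeezes out BP_produkts product actors.
; From BeginPlay it loops: a fixed two-second delay, then the Izpiešana timeline drives the actor's Z scale through its Saspiešana track for a squash animation.
; When the timeline finishes, it spawns a product at the root component's location and restarts the cycle.
; A random-interval node (Minrandom to Maxrandom) is left unconnected.
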(event Collision|EventActorBeginOverlap
  (params (OtherActor :type Actor%20Object%20Reference)))

(event EventBeginPlay
  (Utilities|FlowControl|Delay 2.0 :!label _label)
  (bind _saspiešana (Timeline|izpiešana PlayFromStart)
    (:Update
      (Transformation|SetActorScale3D (Math|Vector|MakeVector 1.0 1.0 _saspiešana)))
    (:Finished
      (Game|SpawnActorfromClass "/Game/KristianaGraumane/02Rupnica/BP/BP_produkts.BP_produkts_C" (Math|Conversions|ToTransform(Vector) (Transformation|GetWorldLocation (Variables|Default|GetDefaultSceneRoot))) "Undefined" 0 0)
      (goto _label))))

(event EventTick
  (params (DeltaSeconds :type Float%20%28single-precision%29)))

(fn ConstructionScript)