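; BP_izmetejs is an ejector that endlessly spawns BP_Produkts actors at its Cube's location at unpredictable intervals.
; From BeginPlay, a loop waits a random time between the Minrandom and Maxrandom variables, then spawns after a further half-second delay before repeating.
; Alongside each spawn delay, the Izspieshana timeline drives the actor's Z scale to animate a squeeze-out effect.
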(event Collision|EventActorBeginOverlap
  (params (OtherActor :type Actor%20Object%20Reference)))

(event EventBeginPlay
  ;[1 0.0156 0] Plūsmas sākums. Palaižas vienu reizi kad sākas spēle
  (Utilities|FlowControl|Delay (Math|Random|RandomFloatinRange (Math|Conversions|ToFloat(Integer) (Variables|Default|Getminrandom)) (Math|Conversions|ToFloat(Integer) (Variables|Default|Getmaxrandom))) :!label _label)
  ;[1 1 1] Sadala plūsmu
  (Utilities|FlowControl|Sequence
    (:then_0
      (Utilities|FlowControl|Delay 0.5)
      ;[0 0.2693 1] Ģenerē BP produktu norādītajā vietā
      (Game|SpawnActorfromClass "/Game/_Piemieri/02Rupnica/BP/BP_Produkts.BP_Produkts_C" (Math|Conversions|ToTransform(Vector) (Transformation|GetWorldLocation (Variables|Default|GetCube))) "Undefined" 0 0)
      (goto _label))
    (:then_1
      ;[1 0.8697 0.1686] Timeline - maina vērtību laikā (animācija). Var pieshķirt raksturu caur "curve editor". Animēto vērtību ievieto vektora z asī un maina izvēlētā "Actor" jeb BP Scale (izmēru) laikā.
      (bind _saspiesana (Timeline|Izspieshana PlayFromStart)
        (:Update
          (Transformation|SetActorScale3D (Math|Vector|MakeVector 1.0 1.0 _saspiesana)))))))

(fn ConstructionScript)