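; BP_izmetejs is a factory ejector actor that repeatedly spawns BP_produktsz products at its Sphere component.
; From BeginPlay it runs an endless loop, starting a squash Timeline that animates the actor's Z scale while a fixed delay counts down to the next spawn.
; The random delay opening each cycle has a zero range, so it adds no intended variation.
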(event Collision|EventActorBeginOverlap
  (params (OtherActor :type Actor%20Object%20Reference)))

(event EventTick
  (params (DeltaSeconds :type Float%20%28single-precision%29)))

(event EventBeginPlay
  (Utilities|FlowControl|Delay (Math|Random|RandomFloatinRange (Math|Conversions|ToFloat(Integer) 0) (Math|Conversions|ToFloat(Integer) 0)) :!label _label)
  (Utilities|FlowControl|Sequence
    (:then_0
      (Utilities|FlowControl|Delay 4.2)
      (Game|SpawnActorfromClass "/Game/KasparsGobins/02Rupnica/BP/BP_produktsz.BP_produktsz_C" (Math|Conversions|ToTransform(Vector) (Transformation|GetWorldLocation (Variables|Default|GetSphere))) "Undefined" 0 0)
      (goto _label))
    (:then_1
      (bind _saspiesana (Timeline|Timeline PlayFromStart)
        (:Update
          (Transformation|SetActorScale3D (Math|Vector|MakeVector 1.0 1.0 _saspiesana)))))))

(fn ConstructionScript)