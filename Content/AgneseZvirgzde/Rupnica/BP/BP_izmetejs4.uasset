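; BP_izmetejs4 is an ejector actor that repeatedly spawns BP_Produkts3 products in what appears to be a factory scene.
; Tick starts a random delay between Minrandom and Maxrandom, then the Izspie timeline animates the actor's Z scale as a squash-and-stretch effect.
; When the timeline finishes, it spawns a product at the Cube component's world location and loops back to the delay.
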(event Collision|EventActorBeginOverlap
  (params (OtherActor :type Actor%20Object%20Reference)))

(event EventTick
  (params (DeltaSeconds :type Float%20%28single-precision%29))
  (Utilities|FlowControl|Delay (Math|Random|RandomFloatinRange (Variables|Default|GetMinrandom\) (Variables|Default|GetMaxrandom)) :!label _label)
  (bind _saspuie (Timeline|izspie PlayFromStart)
    (:Update
      (Transformation|SetActorScale3D (Math|Vector|MakeVector 1.0 1.0 _saspuie)))
    (:Finished
      (Game|SpawnActorfromClass "/Game/AgneseZvirgzde/Rupnica/BP/BP_Produkts3.BP_Produkts3_C" (Math|Conversions|ToTransform(Vector) (Transformation|GetWorldLocation (Variables|Default|GetCube))) "Undefined" 0 0)
      (goto _label))))

(fn ConstructionScript)